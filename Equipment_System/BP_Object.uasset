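; BP_Object is a world item pickup that hands its item to the third-person character on touch.
; The construction script looks up the row referenced by ItemData in its data table and sets the static mesh from it.
; When BP_ThirdPersonCharacter overlaps the collision capsule, the pickup passes ItemData through EquipBowMessage and destroys itself.
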(event `self.Collision Capsule.OnComponentBeginOverlap`
  (params (OverlappedComponent :type "PrimitiveComponent Object Reference") (OtherActor :type "Actor Object Reference") (OtherComp :type "PrimitiveComponent Object Reference") (OtherBodyIndex :type Integer) (bFromSweep :type Boolean) (SweepResult :type "HitResult Structure (by ref)"))
  (bind _asbp_third_person_character (cast `/Game/ThirdPerson/Blueprints/BP_ThirdPersonCharacter` OtherActor))
  (message `/Game/Blueprints/BPI_Equip.EquipBow` _asbp_third_person_character (`self.itemData`))
  (`self.K2_DestroyActor`))

(fn `UserConstructionScript`
  (bind _itemdata (`self.itemData`))
  (bind _returnvalue (`|GetDataTableRow` (break `DataTableRowHandle` (break `/Game/Equipment_System/S_Slots` _itemdata)) (`.RowName` (break `DataTableRowHandle` (break `/Game/Equipment_System/S_Slots` _itemdata))))
    (:`then`
      (`StaticMeshComponent.SetStaticMesh` (`self.StaticMesh`) (`.StaticMesh_8_6E67643A4AD91B4D04C729BF70C57859` (break `/Game/Equipment_System/S_Objects` _returnvalue))))))