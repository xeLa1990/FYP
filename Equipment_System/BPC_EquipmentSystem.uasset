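; Actor component for the player character's equipment system, toggling an equipment menu and holding a list of object items.
; The menu input creates or removes the W_Equipment widget, switching cursor, input mode and character movement.
; AddObject appends item data to ObjectSlots, and a debug key prints their row names.
; A forward sphere-trace pickup that would add and destroy BP_Objects is present but disconnected.
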(event Input|EnhancedActionEvents|EnhancedInputActionIA_Interact
  (params (ActionValue :type Boolean) (ElapsedSeconds :type Float%20%28double-precision%29) (TriggeredSeconds :type Float%20%28double-precision%29) (InputAction :type Input%20Action%20Object%20Reference :default "/Game/ThirdPerson/Input/Actions/IA_Interact.IA_Interact"))
  ;[1 1 1] Pick Up Trace
)

(event Input|EnhancedActionEvents|EnhancedInputActionIA_EquipmentMenu
  (params (ActionValue :type Boolean) (ElapsedSeconds :type Float%20%28double-precision%29) (TriggeredSeconds :type Float%20%28double-precision%29) (InputAction :type Input%20Action%20Object%20Reference :default "/Game/ThirdPerson/Input/Actions/IA_EquipmentMenu.IA_EquipmentMenu"))
  (bind _returnvalue (Game|GetPlayerController 0))
  ;[1 1 1] Eqipment Menu Panel
  (:Started
    (if (not (Variables|Default|GetisMenuOpen))
      (Variables|Default|SetisMenuOpen true)
      (bind _returnvalue_2 (UserInterface|CreateWidget "/Game/UI/Equipment/W_Equipment.W_Equipment_C"))
      (bind _output_get (Variables|Default|SetEquipment%20Widget _returnvalue_2))
      (UserInterface|Viewport|AddtoViewport _output_get 0)
      (Variables|/Script/Engine.PlayerController|SetbShowMouseCursor _returnvalue true)
      (Input|SetInputModeGameandUI _returnvalue (Variables|Default|GetEquipment%20Widget) "DoNotLock" true false)
      (bind _asbp_third_person_character (Utilities|Casting|CastToBP_ThirdPersonCharacter (Components|GetOwner)))
      (Pawn|Components|CharacterMovement|SetMovementMode (Variables|/Script/Engine.Character|GetCharacterMovement _asbp_third_person_character) "MOVE_None" 0)
      (else
        (Variables|Default|SetisMenuOpen false)
        (bind _equipment_widget (Variables|Default|GetEquipment%20Widget)
          (:then
            (Widget|RemovefromParent _equipment_widget)
            (Variables|Default|SetEquipment%20Widget 0)
            (Variables|/Script/Engine.PlayerController|SetbShowMouseCursor _returnvalue false)
            (Input|SetInputModeGameOnly _returnvalue false)
            (bind _asbp_third_person_character_2 (Utilities|Casting|CastToBP_ThirdPersonCharacter (Components|GetOwner)))
            (Pawn|Components|CharacterMovement|SetMovementMode (Variables|/Script/Engine.Character|GetCharacterMovement _asbp_third_person_character_2) "MOVE_Walking" 0))
          (:else))))))

(event EventBeginPlay
  (bind _asbp_third_person_character (Utilities|Casting|CastToBP_ThirdPersonCharacter (Components|GetOwner))))

(event Input|KeyboardEvents|DebugKeyH
  (params (Key :type Key%20Structure) (ActionValue :type Input%20Action%20Value%20Structure))
  ;[1 1 1] Pick Up Trace
  (:Pressed
    (for _array_element (Variables|Default|GetobjectSlots)
      (Development|PrintString (Utilities|String|ToString(Name) (.rowname (.item _array_element)))))))

(fn AddObject
  (params (NewItem :type S%20Slots%20Structure%20%28by%20ref%29))
  (Utilities|Array|Add (Variables|Default|GetobjectSlots) NewItem))