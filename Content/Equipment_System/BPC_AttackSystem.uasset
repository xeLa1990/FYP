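; BPC_AttackSystem is a component on BP_ThirdPersonCharacter that handles bow equipping and aiming, with no projectile firing yet.
; Starting IA_Shoot with a bow equips it in hands, sets AimingBow, switches rotation to follow controller yaw and shows a crosshair widget.
; Completing it restores movement-oriented rotation and removes the crosshair after a short delay.
; Q unequips the bow from hands, and debug prints remain on the shoot input.
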(event `self.ReceiveBeginPlay`
  (bind _asbp_third_person_character (cast `/Game/ThirdPerson/Blueprints/BP_ThirdPersonCharacter` (`self.GetOwner`)))
  (set `self.Character` _asbp_third_person_character))

(event `EnhancedInput|/Game/ThirdPerson/Input/Actions/IA_Shoot`
  (params (ActionValue :type Boolean) (ElapsedSeconds :type "Float (double-precision)") (TriggeredSeconds :type "Float (double-precision)") (InputAction :type "InputAction Object Reference" :default "/Game/ThirdPerson/Input/Actions/IA_Shoot.IA_Shoot"))
  (bind _character (`self.Character`))
  (bind _charactermovement (`Character.CharacterMovement` (`self.Character`)))
  (bind _charactermovement_2 (`Character.CharacterMovement` _character))
  (:`Started`
    (if (`self.Has Bow`)
      (`KismetSystemLibrary.PrintString` "Hello")
      (set `self.Has Ball` false)
      (set `self.Aiming Bow` true)
      (`/Game/ThirdPerson/Blueprints/BP_ThirdPersonCharacter.Equip Bow In Hands` _character)
      (set `CharacterMovementComponent.bUseControllerDesiredRotation` true _charactermovement_2)
      (set `CharacterMovementComponent.bOrientRotationToMovement` false _charactermovement_2)
      (bind _returnvalue (`|CreateWidget` "/Game/UI/W_BowCrosshair.W_BowCrosshair_C"))
      (bind _output_get (set `self.Bow Crosshair Widget` _returnvalue))
      (`UserWidget.AddToViewport` _output_get 0)
      (else
        (`KismetSystemLibrary.PrintString` "no bow"))))
  (:`Completed`
    (if (`self.Has Bow`)
      (set `self.Has Ball` false)
      (set `self.Aiming Bow` false)
      (set `CharacterMovementComponent.bUseControllerDesiredRotation` false _charactermovement)
      (set `CharacterMovementComponent.bOrientRotationToMovement` true _charactermovement)
      (`KismetSystemLibrary.Delay` 0.2)
      (bind _bow_crosshair_widget (`self.Bow Crosshair Widget`)
        (:`then`
          (`Widget.RemoveFromParent` _bow_crosshair_widget)
          (set `self.Bow Crosshair Widget` null))
        (:`else`)))))

(event `Key|Q`
  (params (Key :type "Key Structure"))
  (:`Pressed`
    (if (`self.Has Bow`)
      (`/Game/ThirdPerson/Blueprints/BP_ThirdPersonCharacter.Unequip Bow In Hands` (`self.Character`)))))