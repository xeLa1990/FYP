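; Double door that swings open once every referenced target has been hit, apparently by arrows.
; On BeginPlay it binds to each target's hit event, removing that target from the array when hit and printing how many remain.
; When the array empties, two timelines rotate the left and right door meshes outward in opposite yaw directions.
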(event `self.ReceiveBeginPlay`
  (add `/Game/Blueprints/BP_Target.TargetHit` (`self.TargetRef`) (delegate `Open Door`)))

(event `Open Door`
  (params (TargetActor :type "/Game/Blueprints/BP_Target Object Reference") (Arrow :type "/Game/Blueprints/BP_Arrow Object Reference"))
  (bind _targetref (`self.TargetRef`))
  (bind _returnvalue (`KismetArrayLibrary.Array_Length` _targetref))
  (`KismetArrayLibrary.Array_RemoveItem` _targetref TargetActor)
  (if (<= _returnvalue 0)
    (`|ExecutionSequence`
      (:`then_0`
        (bind (_direction _left_door_open) (`Timeline|Left Door Open`)
          (:`Update`
            (`SceneComponent.K2_SetRelativeRotation` (`self.CubeL`) (`KismetMathLibrary.MakeRotator` 0.0 0.0 (`KismetMathLibrary.Lerp` 0.0 135.0 _left_door_open)) false false))))
      (:`then_1`
        (bind (_direction_2 _right_door_open) (`Timeline|Right Door Open`)
          (:`Update`
            (`SceneComponent.K2_SetRelativeRotation` (`self.CubeR`) (`KismetMathLibrary.MakeRotator` 0.0 0.0 (`KismetMathLibrary.Lerp` 0.0 -135.0 _right_door_open)) false false)))))
    (else
      (`KismetSystemLibrary.PrintString` (`KismetStringLibrary.Concat_StrStr` (`KismetStringLibrary.Conv_IntToString` _returnvalue) " remaining.")))))

(fn `UserConstructionScript`)